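; Player controller for the dungeon game that handles movement and horizontal camera input through Enhanced Input.
; BeginPlay registers the IMC_Game mapping context.
; IA_Move drives the controlled pawn relative to the camera, combining its ground-flattened forward vector and its right vector into a normalized direction.
; IA_CameraController adds yaw to the pawn, negating the input when CameraYawInverse is set.
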(event `self.ReceiveBeginPlay`
  (`EnhancedInputSubsystemInterface.AddMappingContext` (pcsubsystem `EnhancedInputLocalPlayerSubsystem` self) "/Game/IMC_Game.IMC_Game" 0 (struct)))

(event `EnhancedInput|/Game/IA_Move`
  (params (ActionValue :type "Vector2D Structure") (ElapsedSeconds :type "Float (double-precision)") (TriggeredSeconds :type "Float (double-precision)") (InputAction :type "InputAction Object Reference" :default "/Game/IA_Move.IA_Move"))
  (bind (_x _y) (`KismetMathLibrary.BreakVector2D` ActionValue))
  (:`Triggered`
    (`Pawn.AddMovementInput` (`self.K2_GetPawn`) (`KismetMathLibrary.Normal` (+ (* (`KismetMathLibrary.Normal` (`KismetMathLibrary.MakeVector` (.x (`self.GetActorForwardVector` (`GameplayStatics.GetPlayerCameraManager` 0))) (.y (`self.GetActorForwardVector` (`GameplayStatics.GetPlayerCameraManager` 0))))) _y) (* (`self.GetActorRightVector` (`GameplayStatics.GetPlayerCameraManager` 0)) _x))) 1.0 false)))

(event `EnhancedInput|/Game/IA_CameraController`
  (params (ActionValue :type "Float (double-precision)") (ElapsedSeconds :type "Float (double-precision)") (TriggeredSeconds :type "Float (double-precision)") (InputAction :type "InputAction Object Reference" :default "/Game/IA_CameraController.IA_CameraController"))
  (:`Triggered`
    (`Pawn.AddControllerYawInput` (`self.K2_GetPawn`) (`KismetMathLibrary.SelectFloat` (* ActionValue -1.0) ActionValue (`self.CameraYawInverse`)))))

(fn `UserConstructionScript`)